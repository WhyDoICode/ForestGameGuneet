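; BP_AnimalManager is a spawner that keeps releasing random animals from two sides, each given a target on the opposite side.
; Tick feeds a latent random Delay, so spawn waves repeat at irregular intervals of a few seconds.
; Each wave calls two mirrored events that pick a random class, a SideA or SideB start actor and an opposite TargetLocation.
; Every spawned actor is added to the Animals collection.
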(event `self.ReceiveBeginPlay`)

(event `self.ReceiveTick`
  (params (DeltaSeconds :type "Float (single-precision)"))
  (`KismetSystemLibrary.Delay` (`KismetMathLibrary.RandomFloatInRange` 0.0 7.0))
  (`self.SpawnAnimal`)
  (`self.SpawnAnimalInverted`))

(event `SpawnAnimal`
  (bind _returnvalue (`|SpawnActorFromClass` (`KismetArrayLibrary.Array_Random` (`self.AnimalToSpawn`)) (`KismetMathLibrary.MakeTransform` (`self.K2_GetActorLocation` (`KismetArrayLibrary.Array_Random` (`self.SideA`)))) "AdjustIfPossibleButAlwaysSpawn" "MultiplyWithRoot" null (`self.K2_GetActorLocation` (`KismetArrayLibrary.Array_Random` (`self.SideB`))) null))
  (`KismetArrayLibrary.Array_Add` (`self.Animals`) _returnvalue))

(event `SpawnAnimalInverted`
  (bind _returnvalue (`|SpawnActorFromClass` (`KismetArrayLibrary.Array_Random` (`self.AnimalToSpawn`)) (`KismetMathLibrary.MakeTransform` (`self.K2_GetActorLocation` (`KismetArrayLibrary.Array_Random` (`self.SideB`)))) "AdjustIfPossibleButAlwaysSpawn" "MultiplyWithRoot" null (`self.K2_GetActorLocation` (`KismetArrayLibrary.Array_Random` (`self.SideA`))) null))
  (`KismetArrayLibrary.Array_Add` (`self.Animals`) _returnvalue))

(fn `UserConstructionScript`)