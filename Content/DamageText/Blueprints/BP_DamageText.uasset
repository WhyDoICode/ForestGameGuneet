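; Actor that displays a floating damage number through a WBP_DamageText widget, shown for all players.
; Init looks up style settings by type and InitCustomSettings takes an override; both route through ALL_ events into ShowText.
; An optional camera line trace destroys the actor when its point is hidden, and optional distance scaling shrinks the text on BeginPlay.
; The actor expires shortly after the widget's finished callback.
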(event `self.ReceiveBeginPlay`
  (bind _returnvalue (`KismetMathLibrary.FClamp` (/ (`self.DistanceToScale`) (`KismetMathLibrary.Vector_Distance` (`self.K2_GetActorLocation` (`GameplayStatics.GetPlayerCharacter` 0)) (`self.K2_GetActorLocation`)))))
  ;[1 1 1] If we go far - text will be smaller
  (if (`self.DecreaseSizeByDistance`)
    (`Widget.SetRenderScale` (`WidgetComponent.GetUserWidgetObject` (`self.Widget`)) (`KismetMathLibrary.MakeVector2D` _returnvalue _returnvalue))))

(event `ALL_DefaultInit`
  (params (Value :type Text) (Type :type "/Game/DamageText/Blueprints/E_DamageTextValueTypes Enum" :default "NewEnumerator0"))
  ;[1 1 1] Show text
  (bind (_isvalid _output) (`self.FindSettings` Type)) ; Find in settings selected type
  (if _isvalid
    (`self.ShowText` Value _output)
    (else
      (`self.K2_DestroyActor`))))

(event `ALL_InitWithOverride`
  (params (Value :type Text) (Settings :type "/Game/DamageText/Blueprints/S_DamageTextType Structure"))
  ;[1 1 1] Show text
  (`self.ShowText` Value Settings))

(event `Init`
  (params (Value :type Text) (Type :type "/Game/DamageText/Blueprints/E_DamageTextValueTypes Enum" :default "NewEnumerator0"))
  ;[1 1 1] Show damage for all players
  (`self.ALL_DefaultInit` Value Type))

(event `ShowText`
  (params (Value :type Text) (Settings :type "/Game/DamageText/Blueprints/S_DamageTextType Structure"))
  ;[1 1 1] Destroy when not visible
  (bind _returnvalue (`self.CheckVisibility`))
  (if _returnvalue
    ;[1 1 1] When type is finded, create and init widget
    (bind _aswbp_damage_text (cast `/Game/DamageText/Blueprints/WBP_DamageText` (`WidgetComponent.GetUserWidgetObject` (`self.Widget`))))
    (add `/Game/DamageText/Blueprints/WBP_DamageText.OnFinished` _aswbp_damage_text (delegate `OnFinishedEvent`))
    (`/Game/DamageText/Blueprints/WBP_DamageText.Init` _aswbp_damage_text Value Settings)
    (else
      (`self.K2_DestroyActor`))))

(event `InitCustomSettings`
  (params (Value :type Text) (OverrideSettings :type "/Game/DamageText/Blueprints/S_DamageTextType Structure"))
  ;[1 1 1] Show damage for all players
  (`self.ALL_InitWithOverride` Value OverrideSettings))

(event `OnFinishedEvent`
  ;[1 1 1] Destroy actor after animation finished
  (`self.SetLifeSpan` 0.5))

(fn `CheckVisibility`
  (returns (ReturnValue :type Boolean))
  (if (`self.HideWhenDamagePointNotVisible`)
    ;[1 1 1] Dont show text when not visible
    (bind (_outhit _returnvalue) (`KismetSystemLibrary.LineTraceSingle` :`Start` (`PlayerCameraManager.GetCameraLocation` (`GameplayStatics.GetPlayerCameraManager` 0)) :`End` (`self.K2_GetActorLocation`) :`TraceChannel` (`self.CheckVisibilityTraceChannel`) :`bTraceComplex` (`self.CheckVisibilityTraceComplex`) :`DrawDebugType` (`self.Draw Debug Type`)))
    (return (not _returnvalue))
    (else
      (return true))))

(fn `FindSettings`
  (params (Type :type "/Game/DamageText/Blueprints/E_DamageTextValueTypes Enum" :default "NewEnumerator0"))
  (returns (IsValid :type Boolean) (Output :type "/Game/DamageText/Blueprints/S_DamageTextType Structure"))
  (locals (Index :type Integer :default 0) (Valid :type Boolean))
  ;[1 1 1] Find in settings selected type
  (for (_array_element _array_index) (`self.Settings`)
    (if (`|EnumEquality` Type (`.Type_2_4DAB2A384444C748D006AA93DB075307` (break `/Game/DamageText/Blueprints/S_DamageTextType` _array_element)))
      (set `local.Index` _array_index)
      (set `local.Valid` true)))
  (if (`local.Valid`)
    (return true (`|GetArrayItem` (`self.Settings`) (`local.Index`)))
    (else
      (return false))))

(fn `UserConstructionScript`)