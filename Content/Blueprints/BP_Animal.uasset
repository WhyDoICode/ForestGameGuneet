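; BP_Animal is an animal pawn that walks to a target location and affects the player's score.
; When the move succeeds or fails and it is not dying, it destroys itself and deducts points.
; Die runs once, stopping movement, playing a death animation, adding time and points through the first-person player controller, then destroying the actor after a delay.
; GameOver forwards to that controller, and capsule overlap only prints a debug message.
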(event `self.ReceiveBeginPlay`
  (`|AIMoveTo` self (`self.TargetLocation`) null 36.0
    (:`OnSuccess`
      _)
    (:`OnFail`
      _))
  (if (not (`self.IsDying`))
    (`self.K2_DestroyActor`)
    (`self.ReducePoints`)))

(event `self.ReceiveTick`
  (params (DeltaSeconds :type "Float (single-precision)")))

(event `self.CapsuleComponent.OnComponentBeginOverlap`
  (params (OverlappedComponent :type "PrimitiveComponent Object Reference") (OtherActor :type "Actor Object Reference") (OtherComp :type "PrimitiveComponent Object Reference") (OtherBodyIndex :type Integer) (bFromSweep :type Boolean) (SweepResult :type "HitResult Structure (by ref)"))
  (`KismetSystemLibrary.PrintString` "I M HIT"))

(event `Die`
  (bind _mesh (`self.Mesh`))
  (`/Engine/EditorBlueprintResources/StandardMacros.DoOnce` false
    (:`Completed`
      (set `self.IsDying` true)
      (`SkeletalMeshComponent.SetAnimation` _mesh (`self.AnimSequence`))
      (`SkeletalMeshComponent.Play` _mesh false)
      (`MovementComponent.StopMovementImmediately` (`self.CharacterMovement`))
      (`SkeletalMeshComponent.SetPlayRate` _mesh (`self.DeathPlayRate`))
      (`self.Bonus`)
      (`KismetSystemLibrary.Delay` 2.0)
      (`self.K2_DestroyActor`))))

(event `Bonus`
  (bind _asbp_first_person_player_controller (cast `/Game/FirstPerson/Blueprints/BP_FirstPersonPlayerController` (`GameplayStatics.GetPlayerController` 0)))
  (set `/Game/FirstPerson/Blueprints/BP_FirstPersonPlayerController.Timer` (+ (`/Game/FirstPerson/Blueprints/BP_FirstPersonPlayerController.Timer` _asbp_first_person_player_controller) (`self.AddTime`)) _asbp_first_person_player_controller)
  (set `/Game/FirstPerson/Blueprints/BP_FirstPersonPlayerController.Points` (+ (`self.Points`) (`/Game/FirstPerson/Blueprints/BP_FirstPersonPlayerController.Points` _asbp_first_person_player_controller)) _asbp_first_person_player_controller))

(event `GameOver`
  (bind _asbp_first_person_player_controller (cast `/Game/FirstPerson/Blueprints/BP_FirstPersonPlayerController` (`GameplayStatics.GetPlayerController` 0)))
  (`/Game/FirstPerson/Blueprints/BP_FirstPersonPlayerController.GameOver` _asbp_first_person_player_controller))

(event `ReducePoints`
  (bind _asbp_first_person_player_controller (cast `/Game/FirstPerson/Blueprints/BP_FirstPersonPlayerController` (`GameplayStatics.GetPlayerController` 0)))
  (set `/Game/FirstPerson/Blueprints/BP_FirstPersonPlayerController.Points` (- (`/Game/FirstPerson/Blueprints/BP_FirstPersonPlayerController.Points` _asbp_first_person_player_controller) (`self.Points`)) _asbp_first_person_player_controller))

(fn `UserConstructionScript`)