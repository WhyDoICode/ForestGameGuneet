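; BP_Wolf is an enemy wolf whose Die event alternates between provoking it and killing it through a FlipFlop.
; The first call runs a DoOnce AI move toward the player pawn, calling GameOver if the wolf reaches it.
; The second plays the death animation, halts movement, calls Bonus and destroys the wolf after a short delay.
; IsDying is set on every call, including the one that starts the chase.
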(event `self.Die`
  (bind _mesh (`self.Mesh`))
  (set `self.IsDying` true)
  (`/Engine/EditorBlueprintResources/StandardMacros.FlipFlop`
    (:`A`
      (`/Engine/EditorBlueprintResources/StandardMacros.DoOnce` false
        (:`Completed`
          (`MovementComponent.StopMovementImmediately` (`self.CharacterMovement`))
          (`|AIMoveTo` self (0.0 0.0 0.0) (`GameplayStatics.GetPlayerPawn` 0) 55.0
            (:`OnSuccess`
              (`self.GameOver`))))))
    (:`B`
      (`SkeletalMeshComponent.SetAnimation` _mesh (`self.AnimSequence`))
      (`SkeletalMeshComponent.Play` _mesh false)
      (`MovementComponent.StopMovementImmediately` (`self.CharacterMovement`))
      (`SkeletalMeshComponent.SetPlayRate` _mesh (`self.DeathPlayRate`))
      (`self.Bonus`)
      (`KismetSystemLibrary.Delay` 2.0)
      (`self.K2_DestroyActor`))))

(fn `UserConstructionScript`
  (`parent.UserConstructionScript`))